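; Shared hero gameplay ability that unequips the weapon carried under a configured tag.
; It plays an unequip montage, waits for an attach gameplay event to fire the handoff, and ends when the montage completes or is interrupted or cancelled.
; The handoff reattaches the weapon to a mesh socket, links the unarmed anim layer, removes the weapon's input mapping, clears the equipped tag and revokes its granted abilities.
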(event Ability|EventActivateAbility
  (|PlayMontageandWaitProxy "None" (Variables|Default|GetUnequip%20Montage) 1.0 "None" true 1.0 0.0 false
    (:then
      (Ability|Tasks|WaitGameplayEvent (Variables|Default|GetAttach%20Event%20Tag) 0
        (:EventReceived
          (CallFunction|UnequipHandle (Class|HeroCombatComponent|GetHeroCarriedWeaponbyTag (Class|VirgoHeroGameplayAbility|GetHeroCombatComponentfromActorInfo) (Variables|Default|GetUnequip%20Weapon%20Tag))))))
    (:OnCompleted
      (Ability|EndAbility :!label _label))
    (:OnInterrupted
      (goto _label))
    (:OnCancelled
      (goto _label))))

(event Ability|EventOnEndAbility
  (params (bWasCancelled :type Boolean)))

(fn UnequipHandle
  (params (InUnequipWeapon :type Virgo%20Hero%20Weapon%20Object%20Reference))
  (Utilities|IsValid InUnequipWeapon
    (:Is%20Valid
      (LocalVariables|SetUnequip%20Weapon%20Data (Variables|/Script/GasTemplate.VirgoHeroWeapon|GetWeaponData InUnequipWeapon))
      (Transformation|AttachComponentToComponent InUnequipWeapon (Variables|/Script/Engine.Character|GetMesh (.As角色 (Utilities|Casting|CastToCharacter (Ability|GetAvatarActorfromActorInfo)))) (Variables|Default|GetTarget%20Socket%20Name) "SnapToTarget" "KeepRelative" "KeepRelative" true)
      (Utilities|FlowControl|Sequence
        (:then_0
          (Components|SkeletalMesh|AnimationBlueprintLinking|LinkAnimClassLayers (Variables|/Script/Engine.Character|GetMesh (Class|VirgoHeroGameplayAbility|GetHeroCharacterfromActorInfo)) (Variables|Default|GetUnarmed%20Anim%20Layer)))
        (:then_1
          (Input|RemoveMappingContext (PlayerController|LocalPlayerSubsystems|GetEnhancedInputLocalPlayerSubsystem (Class|VirgoHeroGameplayAbility|GetHeroControllerfromActorInfo)) (.WeaponInputMappingContext (Utilities|Struct|BreakVirgoHeroWeaponData (LocalVariables|GetUnequip%20Weapon%20Data))) "(bIgnoreAllPressedKeysUntilRelease=True,bForceImmediately=False,bNotifyUserSettings=False)")
          (Variables|/Script/GasTemplate.PawnCombatComponent|SetCurrentEquippedWeaponTag (Class|VirgoHeroGameplayAbility|GetHeroCombatComponentfromActorInfo) ""))
        (:then_2
          (Class|VirgoAbilitySystemComponent|RemoveHeroAbilities (Class|VirgoGameplayAbility|GetVirgoAbilitySystemComponent) (Class|VirgoHeroWeapon|GetGrantedHeroAbilitySpecHandles InUnequipWeapon)))))
    (:Is%20Not%20Valid
      (Development|PrintString "Can't found weapon by Tag"))))