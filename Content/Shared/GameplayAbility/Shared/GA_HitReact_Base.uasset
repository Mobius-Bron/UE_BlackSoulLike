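; Base hit react gameplay ability, activated by an event, that plays a directional reaction montage on the struck actor.
; It picks the montage from a map using dot products of the target's forward and right vectors with the direction to the instigator.
; Frontal hits get one entry, while rear and both side branches all resolve to the same second entry.
; The ability ends when the montage finishes, or after a short delay without one.
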(event Ability|EventOnEndAbility
  (params (bWasCancelled :type Boolean)))

(event Ability|EventActivateAbilityFromEvent
  (params (EventData :type Gameplay%20Event%20Data%20Structure%20%28by%20ref%29))
  (Variables|Default|SetActive%20Event%20Data EventData)
  (if (Variables|Default|GetHas%20Hit%20React%20Montage%20To%20Play)
    (|PlayMontageandWaitProxy "None" (CallFunction|GetHitReactMontage (.Instigator (Utilities|Struct|BreakGameplayEventData (Variables|Default|GetActive%20Event%20Data))) (.Target (Utilities|Struct|BreakGameplayEventData (Variables|Default|GetActive%20Event%20Data)))) 1.0 "None" true 1.0 0.0 false
      (:OnCompleted
        _)
      (:OnBlendOut
        _)
      (:OnInterrupted
        _)
      (:OnCancelled
        _))
    (Ability|EndAbility)
    (else
      (Utilities|FlowControl|Delay 0.2)
      (Ability|EndAbility))))

(fn GetHitReactMontage
  (params (HitActor :type Actor%20Object%20Reference) (OwnerActor :type Actor%20Object%20Reference))
  (bind _returnvalue (Transformation|GetActorLocation HitActor))
  (bind _returnvalue_2 (Transformation|GetActorLocation OwnerActor))
  (bind _returnvalue_3 (Transformation|GetActorForwardVector OwnerActor))
  (bind _returnvalue_4 (- _returnvalue _returnvalue_2))
  (bind _returnvalue_5 (Math|Vector|Normalize _returnvalue_4))
  (bind _returnvalue_6 (Math|Vector|DotProduct _returnvalue_3 _returnvalue_5))
  (if (> _returnvalue_6 0.7)
    (return (.Value (Utilities|Map|Find (Variables|Default|GetHit%20React%20Montage) 1)))
    (elif (< _returnvalue_6 -0.7)
      (return (.Value (Utilities|Map|Find (Variables|Default|GetHit%20React%20Montage) 2)))
      (elif (> (Math|Vector|DotProduct (Transformation|GetActorRightVector OwnerActor) (Math|Vector|Normalize (- (Transformation|GetActorLocation HitActor) (Transformation|GetActorLocation OwnerActor)))) 0.0)
        (return (.Value (Utilities|Map|Find (Variables|Default|GetHit%20React%20Montage) 2)))
        (else
          (return (.Value (Utilities|Map|Find (Variables|Default|GetHit%20React%20Montage) 2))))))))