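; Shared hero gameplay ability that equips a carried weapon.
; It plays an equip montage, waits for an attach gameplay event to fetch the weapon by tag, and ends when the montage completes or is interrupted or cancelled.
; On that event it snaps the weapon to a mesh socket and uses its weapon data to link anim layers, add an input mapping context and grant abilities, storing their handles on the weapon.
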(event Ability|EventActivateAbility
  (|PlayMontageandWaitProxy "None" (Variables|Default|GetEquip%20Montage) 1.0 "None" true 1.0 0.0 false
    (:then
      (Ability|Tasks|WaitGameplayEvent (Variables|Default|GetAttach%20Event%20Tag) 0
        (:EventReceived
          (CallFunction|HandleEquipWeapon (Class|HeroCombatComponent|GetHeroCarriedWeaponbyTag (Class|VirgoHeroGameplayAbility|GetHeroCombatComponentfromActorInfo) (Variables|Default|GetEquip%20Weapon%20Tag))))))
    (:OnCompleted
      (Ability|EndAbility :!label _label))
    (:OnInterrupted
      (goto _label))
    (:OnCancelled
      (goto _label))))

(event Ability|EventOnEndAbility
  (params (bWasCancelled :type Boolean)))

(fn HandleEquipWeapon
  (params (InEquipWeapon :type Virgo%20Hero%20Weapon%20Object%20Reference))
  (Utilities|IsValid InEquipWeapon
    (:Is%20Valid
      (LocalVariables|SetEquip%20Weapon%20Data (Variables|/Script/GasTemplate.VirgoHeroWeapon|GetWeaponData InEquipWeapon))
      (Transformation|AttachComponentToComponent InEquipWeapon (Variables|/Script/Engine.Character|GetMesh (.As角色 (Utilities|Casting|CastToCharacter (Ability|GetAvatarActorfromActorInfo)))) (Variables|Default|GetTarget%20Socket%20Name) "SnapToTarget" "KeepRelative" "KeepRelative" true)
      (Utilities|FlowControl|Sequence
        (:then_0
          (Components|SkeletalMesh|AnimationBlueprintLinking|LinkAnimClassLayers (Variables|/Script/Engine.Character|GetMesh (Class|VirgoHeroGameplayAbility|GetHeroCharacterfromActorInfo)) (.LinkedAnimLayer (Utilities|Struct|BreakVirgoHeroWeaponData (LocalVariables|GetEquip%20Weapon%20Data)))))
        (:then_1
          (Input|AddMappingContext (PlayerController|LocalPlayerSubsystems|GetEnhancedInputLocalPlayerSubsystem (Class|VirgoHeroGameplayAbility|GetHeroControllerfromActorInfo)) (.WeaponInputMappingContext (Utilities|Struct|BreakVirgoHeroWeaponData (LocalVariables|GetEquip%20Weapon%20Data))) 1 "(bIgnoreAllPressedKeysUntilRelease=True,bForceImmediately=False,bNotifyUserSettings=False)"))
        (:then_2
          (bind _outgrantedabilityspechandle (Class|VirgoAbilitySystemComponent|GrantHeroAbilities (Class|VirgoGameplayAbility|GetVirgoAbilitySystemComponent) (.WeaponAbilityToGrant (Utilities|Struct|BreakVirgoHeroWeaponData (LocalVariables|GetEquip%20Weapon%20Data))) (Ability|GetAbilityLevel)))
          (Class|VirgoHeroWeapon|AssignGrantedHeroAbilitySpecHandles InEquipWeapon _outgrantedabilityspechandle))))
    (:Is%20Not%20Valid
      (Development|PrintString "Can't found weapon by Tag"))))