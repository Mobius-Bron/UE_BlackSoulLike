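; Shared Gameplay Ability that spawns a configurable weapon actor for its avatar and attaches it to a socket on the owning component.
; On activation it spawns the weapon class with the avatar as owner and instigator, then snaps it to the socket location.
; It registers the weapon with the pawn combat component by tag, optionally as equipped, then ends.
; EndAbility runs only when the spawn is valid.
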(event Ability|EventActivateAbility
  (bind _returnvalue (Ability|GetAvatarActorfromActorInfo))
  (bind _returnvalue_2 (Game|SpawnActorfromClass (Variables|Default|GetWeapon%20Class%20To%20Spawn) (Math|Transform|MakeTransform "0, 0, 0" "0, 0, 0" "1.000000,1.000000,1.000000") "AdjustIfPossibleButAlwaysSpawn" "MultiplyWithRoot" _returnvalue (.AsPawn (Utilities|Casting|CastToPawn _returnvalue))))
  (Utilities|IsValid _returnvalue_2
    (:Is%20Valid
      (Variables|Default|SetSpawn%20Weapon _returnvalue_2)
      (Transformation|AttachComponentToComponent (Variables|Default|GetSpawn%20Weapon) (Class|GameplayAbility|GetOwningComponentfromActorInfo) (Variables|Default|GetSocket%20Name%20To%20Attach) "SnapToTarget" "KeepRelative" "KeepWorld" true)
      (Class|PawnCombatComponent|RegisterSpawnedWeapon (Class|VirgoGameplayAbility|GetPawnCombatComponentfromActorInfo) (Variables|Default|GetWeapon%20Tag) (Variables|Default|GetSpawn%20Weapon) (Variables|Default|GetRegister%20as%20Equipped%20Weapon))
      (Ability|EndAbility))))

(event Ability|EventOnEndAbility
  (params (bWasCancelled :type Boolean)))