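; Shared gameplay ability that plays a looping attack combo, advancing one montage per activation.
; It plays the montage mapped to AttackCount, then increments the count and clears the pending reset timer, wrapping to 1 past the last entry.
; When the montage completes, blends out, is interrupted or is cancelled, the ability ends and starts a timer that resets the combo after ResetAttackTime.
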(event Custom|Reset%20Attack%20Count
  (Variables|Default|SetAttack%20Count 1))

(event Custom|Do%20Attack
  (Math|Integer|IncrementInt (Variables|Default|GetAttack%20Count)
    (:%20%20
      (Utilities|Time|ClearandInvalidateTimerbyHandle (Variables|Default|GetRest%20Timer))
      (if (> (Variables|Default|GetAttack%20Count) (Variables|Default|GetAttack%20Max%20Num))
        (CallFunction|ResetAttackCount)))))

(event Ability|EventActivateAbility
  (Utilities|FlowControl|Sequence
    (:then_0
      (Variables|Default|SetAttack%20Max%20Num (Utilities|Map|Length (Variables|Default|GetAttack%20Montage%20List)))
      (|PlayMontageandWaitProxy "None" (.Value (Utilities|Map|Find (Variables|Default|GetAttack%20Montage%20List) (Variables|Default|GetAttack%20Count))) 1.0 "None" true 1.0 0.0 true
        (:then
          (CallFunction|DoAttack))
        (:OnCompleted
          (Ability|EndAbility :!label _label)
          (bind _returnvalue (Utilities|Time|SetTimerbyEvent (delegate Custom|Reset%20Attack%20Count) (Variables|Default|GetReset%20Attack%20Time)))
          (Variables|Default|SetRest%20Timer _returnvalue))
        (:OnBlendOut
          (goto _label))
        (:OnInterrupted
          (goto _label))
        (:OnCancelled
          (goto _label))))))

(event Ability|EventOnEndAbility
  (params (bWasCancelled :type Boolean)))